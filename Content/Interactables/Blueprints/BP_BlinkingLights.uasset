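; BP_BlinkingLights is an interactable light prop that switches its mesh from an initial look to an alert look.
; The construction script and BeginPlay both apply InitialMaterial to material slot 0.
; The StartBlinking event swaps that slot to AlerMaterial, with no timer, toggle or revert in the Blueprint itself.
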(event EventBeginPlay
  (Rendering|Material|SetMaterial (Variables|Default|GetMesh) 0 (Variables|Default|GetInitialMaterial)))

(event Collision|EventActorBeginOverlap
  (params (OtherActor :type Actor%20Object%20Reference)))

(event EventTick
  (params (DeltaSeconds :type Float%20%28single-precision%29)))

(event EventStartBlinking
  (Rendering|Material|SetMaterial (Variables|Default|GetMesh) 0 (Variables|Default|GetAlerMaterial)))

(fn ConstructionScript
  (Rendering|Material|SetMaterial (Variables|Default|GetMesh) 0 (Variables|Default|GetInitialMaterial)))