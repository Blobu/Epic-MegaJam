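; BP_Door1 is a key-locked door that opens when a BP_TopDownCharacter holding every required key overlaps its box, otherwise writing a message on that player's GUI.
; Two chained timelines animate the mesh: a push along X, then a combined Y slide and roll.
; After a delay the timelines play in reverse to close it.
; DoOnce gates block re-opening until fully closed and briefly throttle repeated overlap checks.
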(event OnComponentBeginOverlap(Box)
  (params (OverlappedComponent :type Primitive%20Component%20Object%20Reference) (OtherActor :type Actor%20Object%20Reference) (OtherComp :type Primitive%20Component%20Object%20Reference) (OtherBodyIndex :type Integer) (bFromSweep :type Boolean) (SweepResult :type Hit%20Result%20Structure%20%28by%20ref%29))
  (bind _asbp_top_down_character (Utilities|Casting|CastToBP_TopDownCharacter OtherActor))
  (Utilities|FlowControl|DoOnce false
    (:Completed
      (if (CallFunction|CheckforNeededKeys _asbp_top_down_character)
        (CallFunction|OpenDoor)
        (else
          (Default|WriteMessageonScreen (Variables|/Game/TopDown/Blueprints/BP_TopDownCharacter.BP_TopDownCharacter_C|GetMainGUI _asbp_top_down_character) (Variables|Default|GetTextToWriteIfNoKey) (Variables|Default|GetCoded?))))
      (Utilities|FlowControl|Delay 3.0)
      (CallFunction|ResetHitbox))))

(event Custom|OpenDoor
  (bind _doormesh (Variables|Default|GetDoorMesh))
  (bind _doormesh_2 (Variables|Default|GetDoorMesh))
  (bind _relativelocation (Variables|/Script/Engine.SceneComponent|GetRelativeLocation _doormesh))
  (bind _relativelocation_2 (Variables|/Script/Engine.SceneComponent|GetRelativeLocation _doormesh_2))
  (bind _relativerotation (Variables|/Script/Engine.SceneComponent|GetRelativeRotation _doormesh_2))
  (Utilities|FlowControl|DoOnce false
    (:Completed
      (bind (_direction _newtrack_0) (Timeline|PushRotateDoor PlayFromStart)
        (:Update
          (Transformation|SetRelativeLocation _doormesh (Math|Vector|MakeVector _newtrack_0 (.y _relativelocation) (.z _relativelocation)) false false))
        (:Finished
          (switch Utilities|FlowControl|Switch|SwitchonETimelineDirection _direction
            (:Forward
              (bind (_direction_2 _newtrack_0_2) (Timeline|RotateDoor Play)
                (:Update
                  (Transformation|SetRelativeLocationAndRotation (Variables|Default|GetDoorMesh) (Math|Vector|MakeVector (.x _relativelocation_2) (Math|Float|Lerp 0.0 -2.5e+02 _newtrack_0_2) (.z _relativelocation_2)) (Math|Rotator|MakeRotator (Math|Float|Lerp 0.0 -1e+02 _newtrack_0_2) (.pitch _relativerotation) (.yaw _relativerotation)) false false))
                (:Finished
                  (switch Utilities|FlowControl|Switch|SwitchonETimelineDirection _direction_2
                    (:Forward
                      (Utilities|FlowControl|Delay 1e+01)
                      (CallFunction|CloseDoor))
                    (:Backward
                      (CallFunction|MakeDoorGoBack))))))
            (:Backward
              (CallFunction|ResetOpenDoor))))))))

(event Custom|ResetHitbox
  (Utilities|FlowControl|DoOnce false) ; enters at Reset
)

(event Custom|ResetOpenDoor
  (bind _doormesh (Variables|Default|GetDoorMesh))
  (bind _doormesh_2 (Variables|Default|GetDoorMesh))
  (bind _relativelocation (Variables|/Script/Engine.SceneComponent|GetRelativeLocation _doormesh))
  (bind _relativelocation_2 (Variables|/Script/Engine.SceneComponent|GetRelativeLocation _doormesh_2))
  (bind _relativerotation (Variables|/Script/Engine.SceneComponent|GetRelativeRotation _doormesh_2))
  (Utilities|FlowControl|DoOnce false) ; enters at Reset
)

(event Custom|CloseDoor
  (bind _doormesh (Variables|Default|GetDoorMesh))
  (bind _relativelocation (Variables|/Script/Engine.SceneComponent|GetRelativeLocation _doormesh))
  (bind _relativerotation (Variables|/Script/Engine.SceneComponent|GetRelativeRotation _doormesh))
  (bind (_direction _newtrack_0) (Timeline|RotateDoor ReverseFromEnd)
    (:Update
      (Transformation|SetRelativeLocationAndRotation (Variables|Default|GetDoorMesh) (Math|Vector|MakeVector (.x _relativelocation) (Math|Float|Lerp 0.0 -2.5e+02 _newtrack_0) (.z _relativelocation)) (Math|Rotator|MakeRotator (Math|Float|Lerp 0.0 -1e+02 _newtrack_0) (.pitch _relativerotation) (.yaw _relativerotation)) false false))
    (:Finished
      (switch Utilities|FlowControl|Switch|SwitchonETimelineDirection _direction
        (:Forward
          (Utilities|FlowControl|Delay 1e+01)
          (CallFunction|CloseDoor))
        (:Backward
          (CallFunction|MakeDoorGoBack))))))

(event Custom|MakeDoorGoBack
  (bind _doormesh (Variables|Default|GetDoorMesh))
  (bind _doormesh_2 (Variables|Default|GetDoorMesh))
  (bind _relativelocation (Variables|/Script/Engine.SceneComponent|GetRelativeLocation _doormesh))
  (bind _relativelocation_2 (Variables|/Script/Engine.SceneComponent|GetRelativeLocation _doormesh_2))
  (bind _relativerotation (Variables|/Script/Engine.SceneComponent|GetRelativeRotation _doormesh_2))
  (bind (_direction _newtrack_0) (Timeline|PushRotateDoor ReverseFromEnd)
    (:Update
      (Transformation|SetRelativeLocation _doormesh (Math|Vector|MakeVector _newtrack_0 (.y _relativelocation) (.z _relativelocation)) false false))
    (:Finished
      (switch Utilities|FlowControl|Switch|SwitchonETimelineDirection _direction
        (:Forward
          (bind (_direction_2 _newtrack_0_2) (Timeline|RotateDoor Play)
            (:Update
              (Transformation|SetRelativeLocationAndRotation (Variables|Default|GetDoorMesh) (Math|Vector|MakeVector (.x _relativelocation_2) (Math|Float|Lerp 0.0 -2.5e+02 _newtrack_0_2) (.z _relativelocation_2)) (Math|Rotator|MakeRotator (Math|Float|Lerp 0.0 -1e+02 _newtrack_0_2) (.pitch _relativerotation) (.yaw _relativerotation)) false false))
            (:Finished
              (switch Utilities|FlowControl|Switch|SwitchonETimelineDirection _direction_2
                (:Forward
                  (Utilities|FlowControl|Delay 1e+01)
                  (CallFunction|CloseDoor))
                (:Backward
                  (CallFunction|MakeDoorGoBack))))))
        (:Backward
          (CallFunction|ResetOpenDoor))))))

(fn ConstructionScript)

(fn CheckforNeededKeys
  (params (BP_Players :type BP%20Top%20Down%20Character%20Object%20Reference))
  (for _array_element (Variables|Default|GetNeededKeysArray)
    (if (not (Utilities|Array|ContainsItem (Variables|/Game/TopDown/Blueprints/BP_TopDownCharacter.BP_TopDownCharacter_C|GetKeys BP_Players) _array_element))
      (return false)))
  (return true))