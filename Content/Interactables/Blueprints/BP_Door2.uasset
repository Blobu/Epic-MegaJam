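; BP_Door2 is a key-locked sliding double door that opens when a BP_TopDownCharacter enters its trigger box.
; If the character holds every key in NeededKeysArray, a timeline slides the two meshes apart along local Y, then reverses after a delay.
; Otherwise it writes a configurable message to the character's GUI.
; DoOnce gates block retriggering until the door closes and throttle overlap checks with a short cooldown.
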(event OnComponentBeginOverlap(Box)
  (params (OverlappedComponent :type Primitive%20Component%20Object%20Reference) (OtherActor :type Actor%20Object%20Reference) (OtherComp :type Primitive%20Component%20Object%20Reference) (OtherBodyIndex :type Integer) (bFromSweep :type Boolean) (SweepResult :type Hit%20Result%20Structure%20%28by%20ref%29))
  (bind _asbp_top_down_character (Utilities|Casting|CastToBP_TopDownCharacter OtherActor))
  (Utilities|FlowControl|DoOnce false
    (:Completed
      (if (CallFunction|CheckforNeededKeys _asbp_top_down_character)
        (CallFunction|OpenDoor)
        (else
          (Default|WriteMessageonScreen (Variables|/Game/TopDown/Blueprints/BP_TopDownCharacter.BP_TopDownCharacter_C|GetMainGUI _asbp_top_down_character) (Variables|Default|GetTextToWriteIfNoKey) (Variables|Default|GetCoded?))))
      (Utilities|FlowControl|Delay 3.0)
      (CallFunction|ResetHitbox))))

(event Custom|OpenDoor
  (bind _usa_mare_2_2 (Variables|Default|GetUsa_Mare_2_2))
  (bind _doormesh1 (Variables|Default|GetDoorMesh1))
  (bind _relativelocation (Variables|/Script/Engine.SceneComponent|GetRelativeLocation _doormesh1))
  (bind _relativelocation_2 (Variables|/Script/Engine.SceneComponent|GetRelativeLocation _usa_mare_2_2))
  (Utilities|FlowControl|DoOnce false
    (:Completed
      (bind (_direction _newtrack_0) (Timeline|PushRotateDoor PlayFromStart)
        (:Update
          (Transformation|SetRelativeLocation _doormesh1 (Math|Vector|MakeVector (.x _relativelocation) (Math|Float|Lerp 0.0 1e+02 _newtrack_0) (.z _relativelocation)) false false)
          (Transformation|SetRelativeLocation _usa_mare_2_2 (Math|Vector|MakeVector (.x _relativelocation_2) (* (Math|Float|Lerp 0.0 1e+02 _newtrack_0) -1.0) (.z _relativelocation_2)) false false))
        (:Finished
          (switch Utilities|FlowControl|Switch|SwitchonETimelineDirection _direction
            (:Forward
              (Utilities|FlowControl|Delay 1e+01)
              (CallFunction|MakeDoorGoBack))
            (:Backward
              (CallFunction|ResetOpenDoor))))))))

(event Custom|ResetHitbox
  (Utilities|FlowControl|DoOnce false) ; enters at Reset
)

(event Custom|ResetOpenDoor
  (bind _usa_mare_2_2 (Variables|Default|GetUsa_Mare_2_2))
  (bind _doormesh1 (Variables|Default|GetDoorMesh1))
  (bind _relativelocation (Variables|/Script/Engine.SceneComponent|GetRelativeLocation _doormesh1))
  (bind _relativelocation_2 (Variables|/Script/Engine.SceneComponent|GetRelativeLocation _usa_mare_2_2))
  (Utilities|FlowControl|DoOnce false) ; enters at Reset
)

(event Custom|MakeDoorGoBack
  (bind _usa_mare_2_2 (Variables|Default|GetUsa_Mare_2_2))
  (bind _doormesh1 (Variables|Default|GetDoorMesh1))
  (bind _relativelocation (Variables|/Script/Engine.SceneComponent|GetRelativeLocation _doormesh1))
  (bind _relativelocation_2 (Variables|/Script/Engine.SceneComponent|GetRelativeLocation _usa_mare_2_2))
  (bind (_direction _newtrack_0) (Timeline|PushRotateDoor ReverseFromEnd)
    (:Update
      (Transformation|SetRelativeLocation _doormesh1 (Math|Vector|MakeVector (.x _relativelocation) (Math|Float|Lerp 0.0 1e+02 _newtrack_0) (.z _relativelocation)) false false)
      (Transformation|SetRelativeLocation _usa_mare_2_2 (Math|Vector|MakeVector (.x _relativelocation_2) (* (Math|Float|Lerp 0.0 1e+02 _newtrack_0) -1.0) (.z _relativelocation_2)) false false))
    (:Finished
      (switch Utilities|FlowControl|Switch|SwitchonETimelineDirection _direction
        (:Forward
          (Utilities|FlowControl|Delay 1e+01)
          (CallFunction|MakeDoorGoBack))
        (:Backward
          (CallFunction|ResetOpenDoor))))))

(fn ConstructionScript)

(fn CheckforNeededKeys
  (params (BP_Players :type BP%20Top%20Down%20Character%20Object%20Reference))
  (for _array_element (Variables|Default|GetNeededKeysArray)
    (if (not (Utilities|Array|ContainsItem (Variables|/Game/TopDown/Blueprints/BP_TopDownCharacter.BP_TopDownCharacter_C|GetKeys BP_Players) _array_element))
      (return false)))
  (return true))