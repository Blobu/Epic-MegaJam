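; Interaction component that broadcasts interact and overlap events, with optional dialogue and over-the-shoulder camera switching.
; When dialogue is enabled, it walks DA_Dialogue rows by NextRowName, one line per interaction, in a WB_Dialgoue widget.
; Dialogue ends on a flagged row or when the player lacks the next row's keys, then resets to the initial row.
; It also pre-scans the row chain to collect every needed key.
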(event Custom|InteractDialogue
  (params (Target :type BP%20Top%20Down%20Character%20Object%20Reference))
  (Variables|Default|GetPlayer
    (:then
      _)
    (:else
      (Variables|Default|SetPlayer Target)))
  (if (Variables|Default|GetEnd%20Dialogue)
    (Class|BPIDialogue|EndDialogue(Message) (Variables|/Game/TopDown/Blueprints/BP_TopDownCharacter.BP_TopDownCharacter_C|GetWB_Dialogue (Variables|Default|GetPlayer)))
    (Variables|Default|SetEnd%20Dialogue false)
    (bind _wb_dialogue (Variables|Default|GetWB%20Dialogue)
      (:then
        (Widget|RemovefromParent _wb_dialogue)
        (Variables|Default|SetWB%20Dialogue 0))
      (:else
        _))
    (Default|CallStopDialogueInteraction)
    (Variables|Default|SetRow%20Name (Variables|Default|GetInitialRow))
    (else
      (Variables|Default|GetWB%20Dialogue
        (:then
          (bind _returnvalue (Utilities|GetDataTableRow "/Game/TextAndLanguage/Dialogue/DA_Dialogue.DA_Dialogue" (Variables|Default|GetRow%20Name))
            (:then
              (Variables|Default|SetOut%20Row _returnvalue)
              (Class|BPIDialogue|UpdateDialogue(Message) (Variables|Default|GetWB%20Dialogue) (.dialogue (Variables|Default|GetOut%20Row))))))
        (:else
          (bind _returnvalue_2 (UserInterface|CreateWidget "/Game/GUI/WB_Dialgoue.WB_Dialgoue_C"))
          (Variables|/Game/TopDown/Blueprints/BP_TopDownCharacter.BP_TopDownCharacter_C|SetWB_Dialogue (Variables|Default|GetPlayer) _returnvalue_2)
          (UserInterface|Viewport|AddtoViewport _returnvalue_2 0)
          (Variables|Default|SetWB%20Dialogue _returnvalue_2)
          (bind _returnvalue_3 (Utilities|GetDataTableRow "/Game/TextAndLanguage/Dialogue/DA_Dialogue.DA_Dialogue" (Variables|Default|GetRow%20Name))
            (:then
              (Variables|Default|SetOut%20Row _returnvalue_3)
              (Class|BPIDialogue|BeginDialogue(Message) (Variables|Default|GetWB%20Dialogue) (Variables|Default|GetName) (.dialogue (Variables|Default|GetOut%20Row)))))))
      (bind _playerhasneededkeys (CallFunction|CheckforNeededKeys))
      (if _playerhasneededkeys
        (Variables|Default|SetRow%20Name (.nextrowname (Variables|Default|GetOut%20Row)))
        (Variables|Default|SetEnd%20Dialogue (.enddialogue (Variables|Default|GetOut%20Row)))
        (else
          (Variables|Default|SetEnd%20Dialogue true))))))

(event Custom|ToggleDialogueInteractions
  (params (On :type Boolean))
  (if On
    (EventDispatchers|BindEventtoInteractDispatcher (EventDispatchers|CreateEvent :!event Custom|InteractDialogue))
    (bind _keys (CallFunction|GetAllNeededKeys))
    (Variables|Default|SetNeededKeys _keys)
    (else
      (EventDispatchers|UnbindEventfromInteractDispatcher (EventDispatchers|CreateEvent :!event Custom|InteractDialogue)))))

(event Custom|SwitchCameraBack
  (Variables|Default|SetCamOn? false)
  (bind _player (Variables|Default|GetPlayer)
    (:then
      (Default|SwitchCamera _player false "0, 0, 0"))
    (:else)))

(event EventInteract
  (params (PlayerRef :type BP%20Top%20Down%20Character%20Object%20Reference))
  (Default|CallInteractDispatcher PlayerRef)
  (if (Variables|Default|GetSwitchCamera?)
    (Default|SwitchCamera PlayerRef true (Transformation|GetActorLocation (Components|GetOwner)))
    (Variables|Default|SetCamOn? true)))

(event EventForceEndInteraction
  (Variables|Default|SetEnd%20Dialogue false)
  (bind _wb_dialogue (Variables|Default|GetWB%20Dialogue)
    (:then
      (Widget|RemovefromParent _wb_dialogue)
      (Variables|Default|SetWB%20Dialogue 0))
    (:else
      _))
  (Default|CallStopDialogueInteraction)
  (Variables|Default|SetRow%20Name (Variables|Default|GetInitialRow)))

(event EventSetSwitchCameraONforInteractionComponent
  (Variables|Default|SetSwitchCamera? true)
  (EventDispatchers|BindEventtoStopDialogueInteraction (EventDispatchers|CreateEvent :!event Custom|SwitchCameraBack)))

(event EventToggleOverlappingInteractable
  (params (On :type Boolean))
  (Default|CallOverlapped On))

(event EventBeginPlay
  (Variables|Default|SetRow%20Name (Variables|Default|GetInitialRow)))

(fn CheckforNeededKeys
  (bind _returnvalue (Utilities|GetDataTableRow "/Game/TextAndLanguage/Dialogue/DA_Dialogue.DA_Dialogue" (.nextrowname (Variables|Default|GetOut%20Row)))
    (:then
      (for _array_element (.keysneeded _returnvalue)
        (if (not (Utilities|Array|ContainsItem (Variables|/Game/TopDown/Blueprints/BP_TopDownCharacter.BP_TopDownCharacter_C|GetKeys (Variables|Default|GetPlayer)) _array_element))
          (return false)))
      (return true))
    (:RowNotFound
      (return false))))

(fn GetAllNeededKeys
  (LocalVariables|SetRow (Variables|Default|GetInitialRow))
  (bind _returnvalue (Utilities|GetDataTableRow "/Game/TextAndLanguage/Dialogue/DA_Dialogue.DA_Dialogue" (LocalVariables|GetRow) :!label _label)
    (:then
      (for _array_element (.KeysNeeded (Utilities|Struct|BreakS_Dialogue _returnvalue))
        (Utilities|Array|AddUnique (LocalVariables|GetKeys) _array_element))
      (LocalVariables|SetRow (.NextRowName (Utilities|Struct|BreakS_Dialogue _returnvalue)))
      (if (.EndDialogue (Utilities|Struct|BreakS_Dialogue _returnvalue))
        (return (LocalVariables|GetKeys))
        (else
          (goto _label))))
    (:RowNotFound
      (return (LocalVariables|GetKeys)))))

(fn GetIsCameraon
  (return (Variables|Default|GetCamOn?)))