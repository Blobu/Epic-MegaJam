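; BP_PlayButton is an in-world clickable play button that loads the ComputerHub level behind a fade transition.
; It enables input on BeginPlay and swaps Cube1's material as the cursor enters or leaves the Cube component.
; Clicking Cube spawns a WB_ResetTimeTransition widget, plays its fade animation with a Reverse argument, and opens the level when the animation finishes.
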(event OnBeginCursorOver(Cube)
  (params (TouchedComponent :type Primitive%20Component%20Object%20Reference))
  (Rendering|Material|SetMaterial (Variables|Default|GetCube1) 0 "/Game/Interactables/Blueprints/Meshes/M_Switch_Inst.M_Switch_Inst"))

(event OnEndCursorOver(Cube)
  (params (TouchedComponent :type Primitive%20Component%20Object%20Reference))
  (Rendering|Material|SetMaterial (Variables|Default|GetCube1) 0 "/Game/Interactables/Blueprints/Meshes/M_Switch_Inst1.M_Switch_Inst1"))

(event OnClicked(Cube)
  (params (TouchedComponent :type Primitive%20Component%20Object%20Reference) (ButtonPressed :type Key%20Structure :default "None"))
  (bind _returnvalue (UserInterface|CreateWidget "/Game/GUI/WB_ResetTimeTransition.WB_ResetTimeTransition_C"))
  (Default|SetBlackImage _returnvalue false)
  (UserInterface|Viewport|AddtoViewport _returnvalue 0)
  (Default|PlayFadeAnimation _returnvalue "Reverse")
  (Class|UserWidget|BindtoAnimationFinished _returnvalue (Variables|/Game/GUI/WB_ResetTimeTransition.WB_ResetTimeTransition_C|GetFade _returnvalue) (delegate Custom|OpenLevel)))

(event Custom|OpenLevel
  (Game|OpenLevel(byObjectReference) "/Game/Levels/ComputerHub/ComputerHub.ComputerHub"))

(event EventBeginPlay
  (Input|EnableInput (Game|GetPlayerController 0)))

(event Collision|EventActorBeginOverlap
  (params (OtherActor :type Actor%20Object%20Reference)))

(event EventTick
  (params (DeltaSeconds :type Float%20%28single-precision%29)))

(fn ConstructionScript)