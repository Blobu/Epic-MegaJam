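; BP_Tab is a tablet-style pickup that teaches word translations when the top-down character touches it.
; The first overlap with its box plays a one-shot timeline that raises and spins the Tab component.
; When the animation finishes, Translate writes word and translation pairs into DADictionary, the character's MainGUI starts the translation display, and the actor destroys itself.
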(event OnComponentBeginOverlap(Box)
  (params (OverlappedComponent :type Primitive%20Component%20Object%20Reference) (OtherActor :type Actor%20Object%20Reference) (OtherComp :type Primitive%20Component%20Object%20Reference) (OtherBodyIndex :type Integer) (bFromSweep :type Boolean) (SweepResult :type Hit%20Result%20Structure%20%28by%20ref%29))
  (bind _tab (Variables|Default|Gettab))
  (bind _asbp_top_down_character (Utilities|Casting|CastToBP_TopDownCharacter OtherActor))
  (Utilities|FlowControl|DoOnce false
    (:Completed
      (bind _newtrack_0 (Timeline|Timeline PlayFromStart)
        (:Update
          (Transformation|SetRelativeLocation _tab (Math|Vector|MakeVector 0.0 0.0 (Math|Float|Lerp 0.0 1.2e+02 _newtrack_0)) false false)
          (Transformation|AddRelativeRotation _tab (Math|Rotator|MakeRotator 0.0 0.0 (Math|Float|Lerp 0.0 3e+01 _newtrack_0)) false false))
        (:Finished
          (bind _wordstobetranslated (CallFunction|Translate))
          (Default|StartTranslation (Variables|/Game/TopDown/Blueprints/BP_TopDownCharacter.BP_TopDownCharacter_C|GetMainGUI _asbp_top_down_character) _wordstobetranslated)
          (Actor|DestroyActor))))))

(event EventBeginPlay)

(event Collision|EventActorBeginOverlap
  (params (OtherActor :type Actor%20Object%20Reference)))

(event EventTick
  (params (DeltaSeconds :type Float%20%28single-precision%29)))

(fn ConstructionScript)

(fn Translate
  (bind _wordstobetranslated (Variables|Default|GetWordsToBeTranslated))
  (for (_array_element _array_index) _wordstobetranslated
    (Utilities|Map|Add (Variables|/Game/TextAndLanguage/Language/PDA_Language.PDA_Language_C|GetWords (Variables|Default|GetDA_dictionary)) _array_element (Utilities|Array|Get(acopy) (Variables|Default|GetTranslatedVersion) _array_index))
    (return _wordstobetranslated))
  (return _wordstobetranslated))