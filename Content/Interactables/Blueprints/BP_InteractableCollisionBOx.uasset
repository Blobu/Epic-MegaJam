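; Interactable collision box actor that pairs an interact component with a popup prompt widget showing an image.
; On BeginPlay it clears the component's name, enables dialogue interactions, binds an event to the component's overlap notification and sets the popup image.
; ToggleInteraction shows or hides the prompt widget.
; The box's own begin-overlap handler only casts to the top-down character, with no action after it.
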(event OnComponentBeginOverlap(Box)
  (params (OverlappedComponent :type Primitive%20Component%20Object%20Reference) (OtherActor :type Actor%20Object%20Reference) (OtherComp :type Primitive%20Component%20Object%20Reference) (OtherBodyIndex :type Integer) (bFromSweep :type Boolean) (SweepResult :type Hit%20Result%20Structure%20%28by%20ref%29))
  (Utilities|Casting|CastToBP_TopDownCharacter OtherActor))

(event EventBeginPlay
  (bind _bpc_interact (Variables|Default|GetBPC_Interact))
  (Variables|/Game/Interactables/Blueprints/BPC_Interact.BPC_Interact_C|SetName _bpc_interact " ")
  (Default|ToggleDialogueInteractions _bpc_interact true)
  (EventDispatchers|BindEventtoOverlapped _bpc_interact (EventDispatchers|CreateEvent :!event ToggleInteraction))
  (Class|BPIInteractionPopup|SetPopupImage(Message) (Variables|Default|GetWB_Interactable) "/Game/GUI/Image/Img_E.Img_E"))

(fn ConstructionScript)

(fn ToggleInteraction
  (params (On :type Boolean))
  (Rendering|SetVisibility (Variables|Default|GetWB_Interactable) On false))