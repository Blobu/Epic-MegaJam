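; NPC character that supports dialogue interaction, tracks a new-quest flag and is driven by an AIC_NPC_Base AI controller.
; BPCInteract dispatchers are bound on BeginPlay, and a widget popup can show the interaction key image.
; Starting an interaction saves and switches the state, stopping restores it, and state changes are pushed to the controller's blackboard.
; Movement type selects walk speed, and quest notifications matching the component's NeededKeys set the new-quest flag.
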(event EventShowPopup
  (params (Visibility :type Boolean) (NewParam :type Texture%20Object%20Reference))
  (bind _wb_interactable (Variables|Default|GetWB_Interactable))
  (Rendering|SetVisibility _wb_interactable Visibility false)
  (if Visibility
    (Class|BPIInteractionPopup|SetPopupImage(Message) (UserInterface|GetWidget _wb_interactable) NewParam)))

(event EventSetMovementSpeed
  (params (MovementType :type E_MovementSpeed%20Enum :default "NewEnumerator0"))
  (Variables|/Script/Engine.CharacterMovementComponent|SetMaxWalkSpeed (Variables|Character|GetCharacterMovement) (Utilities|Select :Index MovementType :NewEnumerator0 1.5e+02 :NewEnumerator1 2.5e+02 :NewEnumerator4 5e+02)))

(event EventNotifiNewQuestNPC
  (params (NewQuest :type E_Progression%20Enum :default "NewEnumerator0"))
  (if (Utilities|Array|ContainsItem (Variables|/Game/Interactables/Blueprints/BPC_Interact.BPC_Interact_C|GetNeededKeys (Variables|Default|GetBPC_Interact)) NewQuest)
    (Variables|Default|SetNewQuest true)))

(event EventBeginPlay
  (bind _bpc_interact (Variables|Default|GetBPC_Interact))
  (bind _asaic_npc_base (Utilities|Casting|CastToAIC_NPC_Base (Pawn|GetController)))
  (Variables|Default|SetAICustomController _asaic_npc_base)
  (Default|ToggleDialogueInteractions _bpc_interact true)
  (EventDispatchers|BindEventtoInteractDispatcher _bpc_interact (EventDispatchers|CreateEvent :!event StartInteraction))
  (EventDispatchers|BindEventtoStopDialogueInteraction _bpc_interact (EventDispatchers|CreateEvent :!event StopInteraction))
  (EventDispatchers|BindEventtoOverlapped _bpc_interact (EventDispatchers|CreateEvent :!event ToggleInteractionKeyGUI)))

(event EventUpdateState(BBAswell)
  (params (State :type E_NPCStates%20Enum :default "NewEnumerator0"))
  (if (Utilities|Enum|NotEqual(Enum) State (Variables|Default|GetState))
    (Variables|Default|SetState State)
    (Default|UpdateStatetoBB (Variables|Default|GetAICustomController))))

(fn ConstructionScript)

(fn StartInteraction
  (params (Interactor :type BP%20Top%20Down%20Character%20Object%20Reference))
  (EventDispatchers|UnbindEventfromInteractDispatcher (Variables|Default|GetBPC_Interact) (EventDispatchers|CreateEvent :!event StartInteraction))
  (if (Utilities|Enum|NotEqual(Enum) (Variables|Default|GetState) "NewEnumerator1")
    (Variables|Default|SetOldState (Variables|Default|GetState))
    (CallFunction|UpdateState(BBAswell) "NewEnumerator3")
    (else
      (Variables|Default|SetNewQuest false))))

(fn StopInteraction
  (CallFunction|UpdateState(BBAswell) (Variables|Default|GetOldState))
  (EventDispatchers|BindEventtoInteractDispatcher (Variables|Default|GetBPC_Interact) (EventDispatchers|CreateEvent :!event StartInteraction)))

(fn ToggleInteractionKeyGUI
  (params (On :type Boolean))
  (CallFunction|ShowPopup On "/Game/GUI/Image/Img_E.Img_E"))

(fn GetHasNewQuests
  (return (Variables|Default|GetNewQuest)))

(fn GetState
  (return (Variables|Default|GetState)))