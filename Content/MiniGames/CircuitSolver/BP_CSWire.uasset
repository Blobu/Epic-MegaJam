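; BP_CSWire is a wire in the circuit solver minigame, tracking its current against a target.
; Construction builds spline meshes in fixed-length sections, places the voltmeter widget at the spline's end and offsets a cube to mark the target.
; AddCurrent updates the voltmeter bar and, on exactly hitting the target, fires Success once.
; Success reports the result and key to the player character and optionally passes a streaming level to the game mode.
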(event Custom|Success
  (bind _returnvalue (Actor|GetActorOfClass "/Game/TopDown/Blueprints/BP_TopDownCharacter.BP_TopDownCharacter_C"))
  (Default|MiniGameResult _returnvalue true (Variables|Default|GetMessageToWriteOnSuccess) (Variables|Default|GetMessageCoded?) (Variables|Default|GetWinableKey))
  (if (not (Utilities|Array|IsEmpty (Variables|Default|GetAddStreamingLevelOnSuccess)))
    (Class|BPILevelCorruption|AddLevelCorruption(Message) (Game|GetGameMode) (Variables|Default|GetAddStreamingLevelOnSuccess))))

(event EventBeginPlay
  (bind _aswb_circuit_solver (Utilities|Casting|CastToWB_CircuitSolver (UserInterface|GetWidget (Variables|Default|GetWB_Voltmeter))))
  (Variables|Default|SetAs%20WB%20Circuit%20Solver _aswb_circuit_solver)
  (Default|SetProgressBar (Variables|Default|GetAs%20WB%20Circuit%20Solver) (/ (Variables|Default|GetInitialCurrent) (Variables|Default|GetMaxCurrent))))

(event EventAddCurrent
  (params (Ammount :type Float%20%28double-precision%29))
  (bind _output_get (Variables|Default|SetInitialCurrent (+ (Variables|Default|GetInitialCurrent) Ammount)))
  (Default|SetProgressBar (Variables|Default|GetAs%20WB%20Circuit%20Solver) (/ _output_get (Variables|Default|GetMaxCurrent)))
  (if (== _output_get (Variables|Default|GetTarget))
    (Utilities|FlowControl|DoOnce false
      (:Completed
        (CallFunction|Success)))))

(fn ConstructionScript
  (bind _spline (Variables|Default|GetSpline))
  (for _index (range 0 (Math|Float|Truncate (/ (Spline|GetSplineLength (Variables|Default|GetSpline)) (Variables|Default|GetSectionLength))))
    (Variables|Default|SetIndex _index)
    (bind _returnvalue (AddComponent|AddSplineMeshComponent false))
    (Components|StaticMesh|SetStaticMesh _returnvalue (Variables|Default|GetSplineMesh))
    (SplineMesh|SetForwardAxis _returnvalue "X" true)
    (SplineMesh|SetStartandEnd _returnvalue (.Position (CallFunction|GetPosandTang (Variables|Default|GetIndex))) (.Tangent (CallFunction|GetPosandTang (Variables|Default|GetIndex))) (.Position (CallFunction|GetPosandTang (+ (Variables|Default|GetIndex) 1))) (.Tangent (CallFunction|GetPosandTang (+ (Variables|Default|GetIndex) 1))) true :!class /Script/Engine.SplineMeshComponent))
  (Transformation|SetRelativeTransform (Variables|Default|GetWB_Voltmeter) (Math|Transform|MakeTransform (+ (Spline|GetLocationatSplinePoint _spline (- (Spline|GetNumberOfSplinePoints _spline) 1) "Local") (Variables|Default|GetUIOffset)) (Variables|Default|GetUIRotation) (Variables|Default|GetUIScale)) false false)
  (Transformation|SetRelativeLocation (Variables|Default|GetCube) (Math|Vector|MakeVector 0.0 0.0 (Math|Float|Lerp -2.5e+02 2.5e+02 (/ (Variables|Default|GetTarget) (Variables|Default|GetMaxCurrent)))) false false))

(fn GetPosandTang
  (params (Index :type Integer))
  (bind _sectionlength (Variables|Default|GetSectionLength))
  (bind _spline (Variables|Default|GetSpline))
  (bind _returnvalue (* Index _sectionlength))
  (return (Spline|GetLocationatDistanceAlongSpline _spline _returnvalue "Local") (Math|Vector|ClampVectorSize (Spline|GetTangentatDistanceAlongSpline _spline _returnvalue "Local") 0.0 (Variables|Default|GetSectionLength))))