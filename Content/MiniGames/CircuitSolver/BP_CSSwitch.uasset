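; BP_CSSwitch is a clickable lever switch for the CircuitSolver minigame that changes the current on the wires it touches.
; On BeginPlay it enables input, sends each BP_CSWire overlapping its Box a current value for the initial state and poses the lever to match.
; Clicking the Box flips the state, sends those wires the signed on/off difference and plays or reverses a timeline that rotates the lever.
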(event OnClicked(Box)
  (params (TouchedComponent :type Primitive%20Component%20Object%20Reference) (ButtonPressed :type Key%20Structure :default "None"))
  (bind _addcurrenton (Variables|Default|GetAddCurrentOn))
  (bind _removecurrenoff (Variables|Default|GetRemoveCurrenOff))
  (Variables|Default|SetInitialStatus%28On/Off%29 (not (Variables|Default|GetInitialStatus%28On/Off%29)))
  (for _array_element (Collision|GetOverlappingActors (Variables|Default|GetBox) "/Game/MiniGames/CircuitSolver/BP_CSWire.BP_CSWire_C" :!class /Script/Engine.PrimitiveComponent)
    (Class|BPICircuitSolver|AddCurrent(Message) _array_element (select (Variables|Default|GetInitialStatus%28On/Off%29) (+ _removecurrenoff _addcurrenton) (- (* _removecurrenoff -1.0) _addcurrenton))))
  (if (Variables|Default|GetInitialStatus%28On/Off%29)
    (bind _newtrack_0 (Timeline|LeverAnim Play)
      (:Update
        (Transformation|SetRelativeRotation (Variables|Default|GetPowerSwitchLever) (Math|Rotator|MakeRotator 0.0 (Math|Float|Lerp 0.0 -1.8e+02 _newtrack_0) 0.0) false false)))
    (else
      (Timeline|LeverAnim Reverse))))

(event EventBeginPlay
  (Input|EnableInput (Game|GetPlayerController 0))
  (for _array_element (Collision|GetOverlappingActors (Variables|Default|GetBox) "/Game/MiniGames/CircuitSolver/BP_CSWire.BP_CSWire_C" :!class /Script/Engine.PrimitiveComponent)
    (Class|BPICircuitSolver|AddCurrent(Message) _array_element (select (Variables|Default|GetInitialStatus%28On/Off%29) (Variables|Default|GetAddCurrentOn) (* (Variables|Default|GetRemoveCurrenOff) -1.0))))
  (Transformation|SetRelativeRotation (Variables|Default|GetPowerSwitchLever) (Math|Rotator|MakeRotator 0.0 (select (Variables|Default|GetInitialStatus%28On/Off%29) -1.8e+02 0.0) 0.0) false false))

(fn ConstructionScript)