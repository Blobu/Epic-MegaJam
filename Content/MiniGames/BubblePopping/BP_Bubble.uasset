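; BP_Bubble is a bubble actor for the bubble popping minigame that pops when the top-down character's capsule overlaps its collision.
; On overlap it calls BubblePop on the character, then runs its own Pop event.
; Pop zeroes one custom primitive data float on the sphere and drives another from a timeline, then destroys the actor after a short delay.
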(event OnComponentBeginOverlap(Collision)
  (params (OverlappedComponent :type Primitive%20Component%20Object%20Reference) (OtherActor :type Actor%20Object%20Reference) (OtherComp :type Primitive%20Component%20Object%20Reference) (OtherBodyIndex :type Integer) (bFromSweep :type Boolean) (SweepResult :type Hit%20Result%20Structure%20%28by%20ref%29))
  (bind _ascapsule_collision (Utilities|Casting|CastToCapsuleComponent OtherComp))
  (bind _asbp_top_down_character (Utilities|Casting|CastToBP_TopDownCharacter (Components|GetOwner _ascapsule_collision)))
  (Default|BubblePop _asbp_top_down_character)
  (CallFunction|Pop))

(event Custom|Pop
  (Rendering|Material|SetCustomPrimitiveDataFloat (Variables|Default|GetSphere) 1 0.0)
  (bind _newtrack_0 (Timeline|PopingTimeline PlayFromStart)
    (:Update
      (Rendering|Material|SetCustomPrimitiveDataFloat (Variables|Default|GetSphere) 0 _newtrack_0))
    (:Finished
      (Utilities|FlowControl|Delay 0.2)
      (Actor|DestroyActor))))

(event EventBeginPlay
  (bind _sphere (Variables|Default|GetSphere))
  (Rendering|Material|SetCustomPrimitiveDataFloat _sphere 0 1.0)
  (Rendering|Material|SetCustomPrimitiveDataFloat _sphere 1 1.0))

(fn ConstructionScript)