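; BP_LineOFCode is a clickable line-of-code actor in the calculator minigame, with a cube and up and down triangle buttons.
; On BeginPlay it enables player input and turns off collision on both triangles.
; Clicking the cube drives a FlipFlop that toggles the triangles' visibility and query collision together.
; Both triangle clicks only print a placeholder "Hello", so the buttons have no real behavior yet.
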(event OnClicked(Cube)
  (params (TouchedComponent :type Primitive%20Component%20Object%20Reference) (ButtonPressed :type Key%20Structure :default "None"))
  (bind _isa (Utilities|FlowControl|FlipFlop)
    (:A
      _)
    (:B
      _))
  (Development|SetHiddeninGame (Variables|Default|GetTriangleDown) _isa false)
  (Collision|SetCollisionEnabled (Variables|Default|GetTriangleUp) (select _isa "NoCollision" "QueryOnly")))

(event OnClicked(TriangleUp)
  (params (TouchedComponent :type Primitive%20Component%20Object%20Reference) (ButtonPressed :type Key%20Structure :default "None"))
  (Development|PrintString "Hello"))

(event OnClicked(TriangleDown)
  (params (TouchedComponent :type Primitive%20Component%20Object%20Reference) (ButtonPressed :type Key%20Structure :default "None"))
  (Development|PrintString "Hello"))

(event EventBeginPlay
  (Input|EnableInput (Game|GetPlayerController 0))
  (Collision|SetCollisionEnabled (Variables|Default|GetTriangleUp) "NoCollision"))

(event Collision|EventActorBeginOverlap
  (params (OtherActor :type Actor%20Object%20Reference)))

(event EventTick
  (params (DeltaSeconds :type Float%20%28single-precision%29)))

(fn ConstructionScript)