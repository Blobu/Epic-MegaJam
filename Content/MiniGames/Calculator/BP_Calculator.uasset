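; Code-ordering puzzle mini-game actor that fills child BP_LineOFCode actors with pseudo-program text, some fixed and the rest reorderable by the player.
; DeclareLine configures each line, stores movable ones in an array and binds their click, selection and timeline events.
; MoveLine, gated by a DoOnce, swaps neighbours in world and array and keeps bounds.
; It then checks every line's correct position, though a win triggers nothing yet.
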(event Custom|MoveLine
  (params (Up? :type Boolean) (LineIndex :type Integer))
  (bind _linesofcode (Variables|Default|GetLinesOfCode))
  (Utilities|FlowControl|DoOnce false
    (:Completed
      (Variables|Default|SetCurrentIndex LineIndex)
      (if Up?
        (if (> (Variables|Default|GetCurrentIndex) 0)
          (Default|ChangeLine (Utilities|Array|Get(acopy) _linesofcode (Variables|Default|GetCurrentIndex)) true (Transformation|GetWorldLocation (Variables|/Game/MiniGames/Calculator/BP_LineOFCode.BP_LineOFCode_C|GetDefaultSceneRoot (Utilities|Array|Get(acopy) _linesofcode (+ (Variables|Default|GetCurrentIndex) -1)))))
          (Default|ChangeLine (Utilities|Array|Get(acopy) _linesofcode (+ (Variables|Default|GetCurrentIndex) -1)) false (Transformation|GetWorldLocation (Variables|/Game/MiniGames/Calculator/BP_LineOFCode.BP_LineOFCode_C|GetDefaultSceneRoot (Utilities|Array|Get(acopy) _linesofcode (Variables|Default|GetCurrentIndex)))))
          (CallFunction|ChangeArray true)
          (bind _success (CallFunction|CheckifYouWin :!label _label))
          (if _success
            _)
          (else
            (CallFunction|ResetTrigger :!label _label_2)))
        (elif (< (Variables|Default|GetCurrentIndex) 4)
          (Default|ChangeLine (Utilities|Array|Get(acopy) _linesofcode (Variables|Default|GetCurrentIndex)) false (Transformation|GetWorldLocation (Variables|/Game/MiniGames/Calculator/BP_LineOFCode.BP_LineOFCode_C|GetDefaultSceneRoot (Utilities|Array|Get(acopy) _linesofcode (+ (Variables|Default|GetCurrentIndex) 1)))))
          (Default|ChangeLine (Utilities|Array|Get(acopy) _linesofcode (+ (Variables|Default|GetCurrentIndex) 1)) true (Transformation|GetWorldLocation (Variables|/Game/MiniGames/Calculator/BP_LineOFCode.BP_LineOFCode_C|GetDefaultSceneRoot (Utilities|Array|Get(acopy) _linesofcode (Variables|Default|GetCurrentIndex)))))
          (CallFunction|ChangeArray false)
          (goto _label)
          (else
            (goto _label_2)))))))

(event Custom|ResetTrigger
  (bind _linesofcode (Variables|Default|GetLinesOfCode))
  (Utilities|FlowControl|DoOnce false) ; enters at Reset
)

(event EventBeginPlay
  (CallFunction|DeclareLine (Variables|Default|GetBP_LineOFCode0) false "computer = true" "(R=0.000000,G=0.467784,B=0.000000,A=1.000000)" "" "(R=0.208637,G=0.407240,B=0.208637,A=1.000000)" 2)
  (CallFunction|DeclareLine (Variables|Default|GetBP_LineOFCode1) false "END" "(R=0.000000,G=0.467784,B=0.000000,A=1.000000)" "" "(R=0.208637,G=0.407240,B=0.208637,A=1.000000)" 4)
  (CallFunction|DeclareLine (Variables|Default|GetBP_LineOFCode2) false "          here we go again" "(R=0.000000,G=0.467784,B=0.000000,A=1.000000)" "show " "(R=0.208637,G=0.407240,B=0.208637,A=1.000000)" 3)
  (CallFunction|DeclareLine (Variables|Default|GetBP_LineOFCode3) true "    computer  true" "(R=0.000000,G=0.467784,B=0.000000,A=1.000000)" "if" "(R=0.208637,G=0.407240,B=0.208637,A=1.000000)")
  (CallFunction|DeclareLine (Variables|Default|GetBP_LineOFCode4) true "      computer" "(R=0.000000,G=0.467784,B=0.000000,A=1.000000)" "kill" "(R=0.208637,G=0.407240,B=0.208637,A=1.000000)")
  (CallFunction|DeclareLine (Variables|Default|GetBP_LineOFCode5) true "" "(R=0.000000,G=0.467784,B=0.000000,A=1.000000)" "else" "(R=0.208637,G=0.407240,B=0.208637,A=1.000000)")
  (CallFunction|DeclareLine (Variables|Default|GetBP_LineOFCode6) false "START" "(R=0.000000,G=0.467784,B=0.000000,A=1.000000)" "" "(R=0.208637,G=0.407240,B=0.208637,A=1.000000)")
  (CallFunction|DeclareLine (Variables|Default|GetBP_LineOFCode7) false "create computer" "(R=0.000000,G=0.467784,B=0.000000,A=1.000000)" "" "(R=0.208637,G=0.407240,B=0.208637,A=1.000000)" 1))

(fn ConstructionScript)

(fn DeclareLine
  (params (LineOfCode :type Child%20Actor%20Component%20Object%20Reference) (Fixed? :type Boolean) (InText :type Text) (Color%20And%20Opacity :type Linear%20Color%20Structure :default "(R=0.000000,G=0.467784,B=0.000000,A=1.000000)") (InTextUncoded :type Text) (ColorUnCodedText :type Linear%20Color%20Structure) (CorrectLineIndex :type Integer))
  (bind _asbp_line_ofcode (Utilities|Casting|CastToBP_LineOFCode (Variables|/Script/Engine.ChildActorComponent|GetChildActor LineOfCode)))
  (Default|SetLineOfCodeOptions _asbp_line_ofcode Fixed? InText Color%20And%20Opacity InTextUncoded ColorUnCodedText)
  (Variables|/Game/MiniGames/Calculator/BP_LineOFCode.BP_LineOFCode_C|SetCorrectLineIndex _asbp_line_ofcode CorrectLineIndex)
  (if Fixed?
    _
    (else
      (bind _returnvalue (Utilities|Array|Add (Variables|Default|GetLinesOfCode) _asbp_line_ofcode))
      (Variables|/Game/MiniGames/Calculator/BP_LineOFCode.BP_LineOFCode_C|SetLineIndex _asbp_line_ofcode _returnvalue)))
  (EventDispatchers|BindEventtoOnArrowClick _asbp_line_ofcode (EventDispatchers|CreateEvent :!event Custom|MoveLine))
  (EventDispatchers|BindEventtoTimelineComplete _asbp_line_ofcode (EventDispatchers|CreateEvent :!event Custom|ResetTrigger))
  (EventDispatchers|BindEventtoHasBeenSelected _asbp_line_ofcode (EventDispatchers|CreateEvent :!event ChangeSelected)))

(fn ChangeArray
  (params (Up :type Boolean))
  (bind _currentindex (Variables|Default|GetCurrentIndex))
  (bind _linesofcode (Variables|Default|GetLinesOfCode))
  (bind _currentindex_2 (Variables|Default|GetCurrentIndex))
  (bind _linesofcode_2 (Variables|Default|GetLinesOfCode))
  (if Up
    (Utilities|Array|Insert _linesofcode (Utilities|Array|Get(acopy) _linesofcode _currentindex_2) (+ _currentindex_2 -1))
    (Utilities|Array|RemoveIndex _linesofcode (+ _currentindex_2 1))
    (else
      (Utilities|Array|Insert _linesofcode_2 (Utilities|Array|Get(acopy) _linesofcode_2 (+ _currentindex 1)) _currentindex)
      (Utilities|Array|RemoveIndex _linesofcode_2 (+ _currentindex 2)))))

(fn ChangeSelected
  (params (NewSelectedLine :type BP%20Line%20OF%20Code%20Object%20Reference))
  (bind _oldselectedline (Variables|Default|GetOldSelectedLine)
    (:then
      (Default|ToggleArrows _oldselectedline false))
    (:else
      _))
  (Variables|Default|SetOldSelectedLine NewSelectedLine))

(fn CheckifYouWin
  (for _array_element (Variables|Default|GetLinesOfCode)
    (if (not (Default|IsintheGoodLine _array_element))
      (return false)))
  (return true))