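; BP_MeteorShower runs the meteor shower in the MeteoritesCrasher minigame, spawning BP_Meteorite actors and resolving success or failure.
; StartMiniGame picks a random count if none is set, then SpawnCicle recursively spawns meteorites at random delays and offsets derived from the Plane component.
; After the last spawn, it polls every second and calls Succeed once no meteorites remain.
; Failed stops spawning and destroys all remaining meteorites.
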(event Custom|StartMiniGame
  (if (== (Variables|Default|GetMeteoritesToSpawn) 0)
    (Variables|Default|SetMeteoritesToSpawn (Math|Random|RandomIntegerinRange 10 15)))
  (CallFunction|SpawnCicle))

(event Custom|SpawnCicle
  (bind _plane (Variables|Default|GetPlane))
  (bind _relativelocation (Variables|/Script/Engine.SceneComponent|GetRelativeLocation _plane))
  (Math|Integer|DecrementInt (Variables|Default|GetMeteoritesToSpawn)
    (:%20%20
      (Game|SpawnActorfromClass "/Game/MiniGames/MeteoritesCrasher/BP_Meteorite.BP_Meteorite_C" (Math|Transform|MakeTransform (Math|Transform|TransformLocation (Transformation|GetActorTransform) (Math|Vector|MakeVector (+ (.y _relativelocation) (Math|Random|RandomFloatinRange -3.2e+03 3.2e+03)) (+ (.x _relativelocation) (Math|Random|RandomFloatinRange -4.5e+03 4.5e+03)) (- (.z _relativelocation) 1e+02))) "0, 0, 0" "1.000000,1.000000,1.000000") "Undefined" "MultiplyWithRoot" 0 0)
      (if (> (Variables|Default|GetMeteoritesToSpawn) 0)
        (Utilities|FlowControl|Delay (Math|Random|RandomFloatinRange 1.0 4.0))
        (CallFunction|SpawnCicle)
        (else
          (if (not (Variables|Default|GetFail)) :!label _label
            (bind _outactors (Actor|GetAllActorsOfClass "/Game/MiniGames/MeteoritesCrasher/BP_Meteorite.BP_Meteorite_C"))
            (if (== (Utilities|Array|Length _outactors) 0)
              (Default|CallSucceed)
              (else
                (Utilities|FlowControl|Delay 1.0)
                (goto _label)))))))))

(event Custom|Failed
  (Variables|Default|SetFail true)
  (Variables|Default|SetMeteoritesToSpawn 0)
  (bind _outactors (Actor|GetAllActorsOfClass "/Game/MiniGames/MeteoritesCrasher/BP_Meteorite.BP_Meteorite_C"))
  (for _array_element _outactors
    (Actor|DestroyActor _array_element)))

(fn ConstructionScript)