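; Turret pawn for the Meteorites Crasher minigame, which the player possesses on interaction to fire at a child-actor BP_MeteorShower.
; Interacting swaps the input mapping context, starts the shower and runs a looping timer that turns the barrel toward the cursor hit point; clicking activates a Niagara bullet effect.
; Once-gated success or failure reports to the player and returns possession.
; Success can grant a key and send a level-corruption message to the game mode.
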(event Custom|Interact
  (params (PlayerRef :type BP%20Top%20Down%20Character%20Object%20Reference))
  (bind _returnvalue (Game|GetPlayerController 0))
  (bind _returnvalue_2 (PlayerController|LocalPlayerSubsystems|GetEnhancedInputLocalPlayerSubsystem))
  (bind _output_get (Variables|Default|SetPlayer%20Ref PlayerRef))
  (EventDispatchers|BindEventtoCancelAll _output_get (EventDispatchers|CreateEvent :!event Custom|FailedMiniGame))
  (CallFunction|ResetResult)
  (Pawn|UnPossess _returnvalue)
  (Pawn|Possess _returnvalue self)
  (Input|RemoveMappingContext _returnvalue_2 "/Game/TopDown/Input/IMC_Default.IMC_Default" "(bIgnoreAllPressedKeysUntilRelease=True,bForceImmediately=False,bNotifyUserSettings=False)")
  (Input|AddMappingContext _returnvalue_2 "/Game/TopDown/Input/IMC_MeteoritesGameMode.IMC_MeteoritesGameMode" 0 "(bIgnoreAllPressedKeysUntilRelease=True,bForceImmediately=False,bNotifyUserSettings=False)")
  (bind _returnvalue_3 (Utilities|Time|SetTimerbyEvent (delegate Custom|FollowCursor) 0.05 true))
  (Variables|Default|SetHandle _returnvalue_3)
  (bind _asbp_meteor_shower (Utilities|Casting|CastToBP_MeteorShower (Variables|/Script/Engine.ChildActorComponent|GetChildActor (Variables|Default|GetBP_MeteorShower))))
  (Default|StartMiniGame _asbp_meteor_shower)
  (Variables|Default|SetAs%20BP%20Meteor%20Shower _asbp_meteor_shower))

(event Custom|Overlapped
  (params (On :type Boolean))
  (Rendering|SetVisibility (Variables|Default|GetWB_InteractionPopup) On false))

(event Custom|FollowCursor
  (bind _returnvalue (Transformation|GetActorLocation))
  (bind _returnvalue_2 (Game|GetPlayerController 0))
  (bind _hitresult (Game|Player|GetHitResultUnderCursorbyChannel _returnvalue_2 "TraceTypeQuery1" true))
  (bind _returnvalue_3 (Math|Rotator|FindLookatRotation _returnvalue (.impactpoint _hitresult)))
  (Transformation|SetRelativeRotation (Variables|Default|GetSM_TankBarrel) (Math|Rotator|MakeRotator 0.0 (.pitch _returnvalue_3) (.yaw _returnvalue_3)) false false))

(event Custom|FailedMiniGame
  (bind _returnvalue (Game|GetPlayerController 0))
  (bind _player_ref (Variables|Default|GetPlayer%20Ref))
  (Utilities|FlowControl|DoOnce true
    (:Completed
      (Default|Failed (Variables|Default|GetAs%20BP%20Meteor%20Shower))
      (Default|MiniGameResult (Variables|Default|GetPlayer%20Ref) false (Variables|Default|GetMessageToWriteOnLose\) (Variables|Default|GetMessagesCoded?) "NewEnumerator0")
      (Utilities|Time|ClearandInvalidateTimerbyHandle (Variables|Default|GetHandle))
      (Pawn|UnPossess _returnvalue)
      (Pawn|Possess _returnvalue _player_ref)
      (Default|SwitchBackController _player_ref))))

(event Custom|SuccedMiniGame
  (bind _returnvalue (Game|GetPlayerController 0))
  (bind _player_ref (Variables|Default|GetPlayer%20Ref))
  (Utilities|FlowControl|DoOnce true
    (:Completed
      (Default|MiniGameResult (Variables|Default|GetPlayer%20Ref) true (Variables|Default|GetMessageToWriteOnSuccess) (Variables|Default|GetMessagesCoded?) (Variables|Default|GetWinableKey))
      (if (Utilities|Array|IsEmpty (Variables|Default|GetAddStreamingLevelOnSuccess))
        _
        (else
          (Class|BPILevelCorruption|AddLevelCorruption(Message) (Game|GetGameMode) (Variables|Default|GetAddStreamingLevelOnSuccess))))
      (Utilities|Time|ClearandInvalidateTimerbyHandle (Variables|Default|GetHandle))
      (Pawn|UnPossess _returnvalue)
      (Pawn|Possess _returnvalue _player_ref)
      (Default|SwitchBackController _player_ref))))

(event Custom|ResetResult
  (bind _returnvalue (Game|GetPlayerController 0))
  (bind _player_ref (Variables|Default|GetPlayer%20Ref))
  (bind _player_ref_2 (Variables|Default|GetPlayer%20Ref))
  (Utilities|FlowControl|Sequence
    (:then_0
      (Utilities|FlowControl|DoOnce true) ; enters at Reset
    )
    (:then_1
      (Utilities|FlowControl|DoOnce true) ; enters at Reset
    )))

(event Input|EnhancedActionEvents|EnhancedInputActionIA_Click
  (params (ActionValue :type Boolean) (ElapsedSeconds :type Float%20%28double-precision%29) (TriggeredSeconds :type Float%20%28double-precision%29) (InputAction :type Input%20Action%20Object%20Reference :default "/Game/TopDown/Input/Actions/IA_Click.IA_Click"))
  (Components|Activation|Activate (Variables|Default|GetNS_BulletEffect) false))

(event EventBeginPlay
  (bind _bpc_interact (Variables|Default|GetBPC_Interact))
  (EventDispatchers|BindEventtoInteractDispatcher _bpc_interact (EventDispatchers|CreateEvent :!event Custom|Interact))
  (EventDispatchers|BindEventtoOverlapped _bpc_interact (EventDispatchers|CreateEvent :!event Custom|Overlapped))
  (bind _asbp_meteor_shower (Utilities|Casting|CastToBP_MeteorShower (Variables|/Script/Engine.ChildActorComponent|GetChildActor (Variables|Default|GetBP_MeteorShower))))
  (EventDispatchers|BindEventtoSucceed _asbp_meteor_shower (EventDispatchers|CreateEvent :!event Custom|SuccedMiniGame)))

(fn ConstructionScript
  (bind _box (Variables|Default|GetBox))
  (Transformation|SetRelativeLocation _box (Variables|Default|GetInteractionBoxOffset) false false)
  (Components|Box|SetBoxExtent _box (Variables|Default|GetInteractionBoxSize) true))