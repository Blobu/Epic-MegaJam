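; BP_Locker is a combination-lock mini-game that succeeds when all its symbol wheels show the right symbol.
; One second after BeginPlay, it counts the BP_Wheel actors overlapping its Box and binds to their RightSymbol events.
; ChangeCorrectSymbols tracks the correct count up or down.
; When an increment reaches the total, it reports success to BP_TopDownCharacter with a message and key setting.
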(event Custom|ChangeCorrectSymbols
  (params (Add :type Boolean))
  (bind _nrofcorrectsymbols (Variables|Default|GetNrOfCorrectSymbols))
  (if Add
    (bind _result (Math|Integer|IncrementInt _nrofcorrectsymbols)
      (:%20%20
        (if (== _result (Variables|Default|GetNrOfSymbols))
          (bind _returnvalue (Actor|GetActorOfClass "/Game/TopDown/Blueprints/BP_TopDownCharacter.BP_TopDownCharacter_C"))
          (Default|MiniGameResult _returnvalue true (Variables|Default|GetMessageToWriteOnSucces) (Variables|Default|GetMessage%20Coded?) (Variables|Default|GetObtain%20Key))
          (Development|PrintString "Hello"))))
    (else
      (Math|Integer|DecrementInt _nrofcorrectsymbols))))

(event EventBeginPlay
  (bind _box (Variables|Default|GetBox))
  (bind _overlappingactors (Collision|GetOverlappingActors _box "/Game/MiniGames/Locker/BP_Wheel.BP_Wheel_C" :!class /Script/Engine.PrimitiveComponent))
  (Utilities|FlowControl|Delay 1.0)
  (Variables|Default|SetNrOfSymbols (Utilities|Array|Length _overlappingactors))
  (for _array_element _overlappingactors
    (bind _asbp_wheel (Utilities|Casting|CastToBP_Wheel _array_element))
    (EventDispatchers|BindEventtoRightSymbol _asbp_wheel (EventDispatchers|CreateEvent :!event Custom|ChangeCorrectSymbols))))

(fn ConstructionScript)