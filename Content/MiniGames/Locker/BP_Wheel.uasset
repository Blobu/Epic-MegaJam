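; One clickable six-faced wheel for a locker minigame, with configurable mesh, material, starting face and correct face.
; Construction script previews the starting face as a pitch in 60-degree steps.
; Arrow clicks step the wrapping face index and play a timeline that lerps rotation, with a DoOnce blocking re-entry until it finishes.
; It then fires CallRightSymbol true on the correct face, or false when leaving it.
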(event OnClicked(UpArrowMesh)
  (params (TouchedComponent :type Primitive%20Component%20Object%20Reference) (ButtonPressed :type Key%20Structure :default "None"))
  (CallFunction|Rotate true))

(event OnClicked(DownArrowMesh)
  (params (TouchedComponent :type Primitive%20Component%20Object%20Reference) (ButtonPressed :type Key%20Structure :default "None"))
  (CallFunction|Rotate false))

(event Custom|Rotate
  (params (Up :type Boolean))
  (Utilities|FlowControl|DoOnce false
    (:Completed
      (Variables|Default|SetOldRotation (Variables|Default|GetNewRotation))
      (Variables|Default|SetNewRotation (+ (Variables|Default|GetNewRotation) (select Up 6e+01 -6e+01)))
      (bind _output_get (Variables|Default|SetInitialFace%281-6%29 (+ (Variables|Default|GetInitialFace%281-6%29) (select Up 1 -1))))
      (if (< _output_get 1)
        (Variables|Default|SetInitialFace%281-6%29 6)
        (bind _newtrack_0 (Timeline|RotateWheel PlayFromStart)
          (:Update
            (Transformation|SetRelativeRotation (Variables|Default|GetWheelStaticMesh) (Math|Rotator|MakeRotator 0.0 (Math|Float|Lerp (Variables|Default|GetOldRotation) (Variables|Default|GetNewRotation) _newtrack_0) 0.0) false false))
          (:Finished
            (CallFunction|ResetAnimation)
            (if (== (Variables|Default|GetInitialFace%281-6%29) (Variables|Default|GetGoodFace%281-6%29))
              (Variables|Default|SetGood true)
              (Default|CallRightSymbol true)
              (elif (Variables|Default|GetGood)
                (Variables|Default|SetGood false)
                (Default|CallRightSymbol false)))))
        (elif (> _output_get 6)
          (Variables|Default|SetInitialFace%281-6%29 1)
          (Timeline|RotateWheel PlayFromStart)
          (else
            (Timeline|RotateWheel PlayFromStart)))))))

(event Custom|ResetAnimation
  (Utilities|FlowControl|DoOnce false) ; enters at Reset
)

(event EventBeginPlay
  (Input|EnableInput (Game|GetPlayerController 0))
  (Variables|Default|SetNewRotation (Math|Conversions|ToFloat(Integer) (* (- (Math|Integer|Clamp(Integer) (Variables|Default|GetInitialFace%281-6%29) 1 6) 1) 60))))

(fn ConstructionScript
  (bind _wheelstaticmesh (Variables|Default|GetWheelStaticMesh))
  (Components|StaticMesh|SetStaticMesh _wheelstaticmesh (Variables|Default|GetWheelMesh))
  (Rendering|Material|SetMaterial _wheelstaticmesh 0 (Variables|Default|GetWheelMaterial))
  (Transformation|SetRelativeRotation (Variables|Default|GetWheelStaticMesh) (Math|Rotator|MakeRotator 0.0 (Math|Conversions|ToFloat(Integer) (* (- (Math|Integer|Clamp(Integer) (Variables|Default|GetInitialFace%281-6%29) 1 6) 1) 60)) 0.0) false false))