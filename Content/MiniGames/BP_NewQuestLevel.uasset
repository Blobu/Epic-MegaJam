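; BP_NewQuestLevel is a trigger box that, on first overlap by the top-down character, reports a successful mini-game result to that character.
; The result carries a message to write, its coded version and an obtain-key value.
; If a streaming level name is set, it also passes that name to the game mode's level corruption message call.
; A DoOnce gate runs before the character cast, so the first overlapping actor of any type consumes it.
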(event OnComponentBeginOverlap(Box)
  (params (OverlappedComponent :type Primitive%20Component%20Object%20Reference) (OtherActor :type Actor%20Object%20Reference) (OtherComp :type Primitive%20Component%20Object%20Reference) (OtherBodyIndex :type Integer) (bFromSweep :type Boolean) (SweepResult :type Hit%20Result%20Structure%20%28by%20ref%29))
  (Utilities|FlowControl|DoOnce false
    (:Completed
      (Development|PrintString "overlap")
      (bind _asbp_top_down_character (Utilities|Casting|CastToBP_TopDownCharacter OtherActor))
      (Default|MiniGameResult _asbp_top_down_character true (Variables|Default|GetMessage%20to%20Write) (Variables|Default|GetMessage%20Coded?) (Variables|Default|GetObtain%20Key))
      (if (not (Utilities|Array|IsEmpty (Variables|Default|GetAddStreamingLevel)))
        (Class|BPILevelCorruption|AddLevelCorruption(Message) (Game|GetGameMode) (Variables|Default|GetAddStreamingLevel))))))

(fn ConstructionScript)