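; BPC_Dialogue is a dialogue component that shows one line of data-table-driven dialogue each time its Interact event fires.
; It looks up the current row and, when found, creates a WB_Dialgoue widget with the speaker's name and line, then adds it to the viewport.
; The row then supplies the next row name, data table and end-dialogue value, so conversations chain across rows and tables.
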(event EventInteract
  (params (PlayerRef :type BP%20Top%20Down%20Character%20Object%20Reference))
  (bind _returnvalue (Utilities|GetDataTableRow (Variables|Default|GetData%20Table) (Variables|Default|GetRow%20Name))
    (:then
      (bind _returnvalue_2 (UserInterface|CreateWidget "/Game/GUI/WB_Dialgoue.WB_Dialgoue_C" 0 (Utilities|Text|ToText(Name) (Variables|Default|GetName)) (.Dialogue (Utilities|Struct|BreakS_Dialogue _returnvalue))))
      (bind _output_get (Variables|Default|SetDialogueWidget _returnvalue_2))
      (UserInterface|Viewport|AddtoViewport _output_get 0)
      (Variables|Default|SetRow%20Name (.Row (Utilities|Struct|BreakS_Dialogue _returnvalue)))
      (Variables|Default|SetData%20Table (.DataTable (Utilities|Struct|BreakS_Dialogue _returnvalue)))
      (Variables|Default|SetEnd%20Dialogue (.EndDialogue (Utilities|Struct|BreakS_Dialogue _returnvalue))))))